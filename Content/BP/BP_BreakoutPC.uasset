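; Player controller for a Breakout game that handles paddle movement, ball launch and pausing.
; The horizontal axis, scaled by a speed variable, feeds movement input along world X to the controlled pawn.
; The launch action calls LaunchBall only once, guarded by a launched flag that this file never resets.
; The pause action pauses the game and adds a newly created pause widget to the viewport.
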(event `self.ReceiveBeginPlay`
  ;[1 1 1] Enable input to controller
  (`self.EnableInput` (`GameplayStatics.GetPlayerController` 0)))

(event `InputAxis|MoveHorizontal`
  (params (AxisValue :type "Float (single-precision)"))
  ;[1 1 1] Handle paddle movement
  (`Pawn.AddMovementInput` (`self.K2_GetPawn`) (`KismetMathLibrary.MakeVector` (* AxisValue (`self.Speed`))) 1.0 false))

(event `InputAction|Pause`
  (params (Key :type "Key Structure"))
  ;[1 1 1] Handle pause key
  (:`Pressed`
    (`GameplayStatics.SetGamePaused` true)
    (bind _returnvalue (`|CreateWidget` "/Game/WBP/WBP_PauseUI.WBP_PauseUI_C"))
    (`UserWidget.AddToViewport` _returnvalue 0)))

(event `InputAction|Launch`
  (params (Key :type "Key Structure"))
  ;[1 1 1] Handle launch ball input
  (:`Pressed`
    (if (not (`self.Ball Launched?`))
      (set `self.Ball Launched?` true)
      (`self.LaunchBall`))))

(fn `UserConstructionScript`)