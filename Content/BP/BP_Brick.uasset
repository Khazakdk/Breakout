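; BP_Brick is a breakable brick that reacts to hits from BP_Ball, as in a Breakout-style game.
; On each ball hit, it adds a fraction of the ball's velocity based on BounceSpeed, a bounce calculation marked as rough, and decrements HitsToBreak.
; At zero hits left it calls its destroyed notification, destroys itself and has a small random chance to spawn a scaled-down BP_Powerup in its place.
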(event `self.SM_Brick.OnComponentHit`
  (params (HitComponent :type "PrimitiveComponent Object Reference") (OtherActor :type "Actor Object Reference") (OtherComp :type "PrimitiveComponent Object Reference") (NormalImpulse :type "Vector Structure") (Hit :type "HitResult Structure (by ref)"))
  ;[1 1 1] rough attempt at mathing out new ball speed, needs work
  (bind _asbp_ball (cast `/Game/BP/BP_Ball` OtherActor))
  (`PrimitiveComponent.SetPhysicsLinearVelocity` (`/Game/BP/BP_Ball.SM_Ball` _asbp_ball) (* (`self.GetVelocity` _asbp_ball) (- (`self.BounceSpeed`) 1.0)) true "None")
  ;[1 1 1] Add damage to brick, destroy if needed, roll powerup chance
  (`/Engine/EditorBlueprintResources/StandardMacros.DecrementInt` (`self.HitsToBreak`)
    (:`  `
      (if (<= (`self.HitsToBreak`) 0)
        (`self.DestroyedNotification`)
        (`self.K2_DestroyActor`)
        (if (< (`KismetMathLibrary.RandomFloatInRange` 0.0 0.99) 0.09)
          (`|SpawnActorFromClass` "/Game/BP/BP_Powerup.BP_Powerup_C" (`KismetMathLibrary.MakeTransform` (`self.K2_GetActorLocation`) (struct) (0.2 0.2 0.2)) "AlwaysSpawn" "OverrideRootScale" null null))))))

(fn `UserConstructionScript`)